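; Blueprint function library for the auto spawner, computing chair placement transforms and per-instance chair colors.
; Square Transform fills a spline outline with a rotated grid, stepping height per row and testing points by ray-crossing parity.
; Other helpers space transforms along a spline with offsets, snap to landscape via line trace, and find HISM instances.
; Color enums map to chair materials, whose "Param" color feeds widgets or instance custom data.
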(fn `Calculate Point Transforms`
  (params (`Offset Spline Details` :type "/Game/fan_spawner/Structs/ST_OffsetSpline Structure (by ref)") (`Offset right` :type "Float (double-precision)") (`Offset Up` :type "Float (double-precision)") (`Mesh Spacing` :type "Float (double-precision)") (`Base Spline` :type "SplineComponent Object Reference") (`__WorldContext object` :type "Object Object Reference"))
  (returns (InstanceTransforms :type "Array of Transform Structure"))
  (locals (L_InstanceTransforms :type "Array of Transform Structure") (L_ReferenceSpline :type "SplineComponent Object Reference") (L_DistanceAlongOffsetSplineAtBasePoints :type "Array of Float (double-precision)") (L_IsUsingBaseSplineAsOffsetSpline :type Boolean) (L_CurrentMeshDistance :type "Float (double-precision)") (L_SplineEndDistance :type "Float (double-precision)") (L_SplineStartDistance :type "Float (double-precision)") (L_MeshSpacing :type "Float (double-precision)") (L_MeshSpacingVar :type "Float (double-precision)") (L_OffsetRightVar :type "Float (double-precision)") (L_MeshesAlwaysVertical :type Boolean) (L_AllowGapSmallerThanSpacing :type Boolean) (L_StartAndEndClearance :type "/Game/fan_spawner/Structs/ST_StartEndClearance Structure") (L_RepeatSettings :type "/Game/fan_spawner/Structs/ST_PointElemRepeatSettings Structure") (L_RepeatOffset :type "Float (double-precision)") (L_OffsetUp :type "Float (double-precision)") (L_OffsetRight :type "Float (double-precision)"))
  (bind (_offsetsplinecomponent _distancealongoffsetsplineatbasepoints _iscornerpoint _isusingbasesplineasoffsetspline) (break `/Game/fan_spawner/Structs/ST_OffsetSpline` `Offset Spline Details`))
  (bind _returnvalue (`KismetMathLibrary.Abs` 0.0))
  (bind _l_referencespline (`local.L_ReferenceSpline`))
  (`KismetArrayLibrary.Array_Clear` (`local.L_InstanceTransforms`))
  (set `local.L_ReferenceSpline` _offsetsplinecomponent)
  (set `local.L_DistanceAlongOffsetSplineAtBasePoints` _distancealongoffsetsplineatbasepoints)
  (set `local.L_IsUsingBaseSplineAsOffsetSpline` _isusingbasesplineasoffsetspline)
  (`|ExecutionSequence`
    (:`then_0`
      ;[1 1 1] Set local variables for easier referencing
      (set `local.L_OffsetRight` `Offset right`)
      (set `local.L_OffsetUp` `Offset Up`)
      (set `local.L_RepeatSettings` (struct))
      (set `local.L_MeshSpacing` `Mesh Spacing`)
      (set `local.L_SplineStartDistance` (`KismetMathLibrary.SelectFloat` (`SplineComponent.GetDistanceAlongSplineAtSplinePoint` (`local.L_ReferenceSpline`) 0) 0.0 (`local.L_IsUsingBaseSplineAsOffsetSpline`)))
      (set `local.L_SplineEndDistance` (`KismetMathLibrary.SelectFloat` (`SplineComponent.GetDistanceAlongSplineAtSplinePoint` _l_referencespline (`self.ValidateStartAndEndPoints` `Base Spline` `__WorldContext object`)) (`SplineComponent.GetSplineLength` _l_referencespline) (`local.L_IsUsingBaseSplineAsOffsetSpline`)))
      (set `local.L_MeshesAlwaysVertical` false)
      (set `local.L_AllowGapSmallerThanSpacing` false))
    (:`then_1`
      ;[1 1 1] Check that Start Distance is smaller than End Distance
      (if (< (`local.L_SplineStartDistance`) (`local.L_SplineEndDistance`))
        ;[1 1 1] This loop controls the Repeating Elements
        (for _index (range 1)
          (set `local.L_RepeatOffset` (+ (* _index 0.0) 1.0))
          ;[1 1 1] Mode 1B - Create mesh instances at regular spacing along the OffsetSpline
          (set `local.L_CurrentMeshDistance` (`local.L_SplineStartDistance`))
          (while (<= (`local.L_CurrentMeshDistance`) (`local.L_SplineEndDistance`))
            (`KismetArrayLibrary.Array_Add` (`local.L_InstanceTransforms`) (`self.GetInstanceTransform` (`local.L_ReferenceSpline`) -1 (`local.L_CurrentMeshDistance`) -1 0.0 true 0.0 0.0 0.0 (`local.L_RepeatOffset`) (`local.L_MeshesAlwaysVertical`) `__WorldContext object` `__WorldContext object`))
            ;;[1 0.3606 0] IMPORTANT - Do not disconnect this from the While Loop
            (set `local.L_CurrentMeshDistance` (+ (`local.L_CurrentMeshDistance`) (`local.L_MeshSpacing`) (`KismetMathLibrary.RandomFloatInRange` (* _returnvalue -1.0) _returnvalue))))
          (if (`local.L_AllowGapSmallerThanSpacing`)
            (`KismetArrayLibrary.Array_Add` (`local.L_InstanceTransforms`) (`self.GetInstanceTransform` (`local.L_ReferenceSpline`) -1 (`local.L_SplineEndDistance`) -1 0.0 true 0.0 0.0 0.0 (`local.L_RepeatOffset`) (`local.L_MeshesAlwaysVertical`) `__WorldContext object` `__WorldContext object`))))
        (return (`local.L_InstanceTransforms`))))))

(fn `ETraceType2ECollisionChannel`
  (params (TraceType :type "ETraceTypeQuery Enum" :default "TraceTypeQuery1"))
  (returns (ReturnValue :type "ECollisionChannel Enum"))
  (locals (Local_traceType :type "ETraceTypeQuery Enum"))
  (set `local.Local_traceType` TraceType)
  (for _index (range (+ (enumcount `ECollisionChannel`) 1))
    (bind _returnvalue (cast `ECollisionChannel` (`KismetMathLibrary.Conv_IntToByte` _index)))
    (if (`KismetStringLibrary.EqualEqual_StrStr` (`|GetEnumeratorNameAsString` (`local.Local_traceType`)) (`|GetEnumeratorNameAsString` _returnvalue))
      (return _returnvalue))))

(fn `FastAlignWithLandscape`
  (params (InTransform :type "Transform Structure (by ref)") (BP_AutoSpawner :type "/Game/fan_spawner/Blueprints/Main_Blueprints/BP_Fan_Spawner Object Reference"))
  (returns (IsSuccess :type Boolean) (ReturnValue :type "Transform Structure"))
  (locals (Local_LandscapeCollisionChannel :type "ETraceTypeQuery Enum") (Local_IsUseParametrs :type Boolean) (Local_SpawnParametrs :type "/Game/fan_spawner/Structs/ST_SpawnParametrs Structure") (Local_Scale :type "Vector Structure"))
  (bind _location (.location InTransform))
  (bind (_outhit _returnvalue) (`KismetSystemLibrary.LineTraceSingle` :`Start` _location :`End` (+ _location (* (`KismetMathLibrary.GetUpVector` (struct :`Yaw` 90.0)) -100000)) :`TraceChannel` (`local.Local_LandscapeCollisionChannel`) :`DrawTime` 100.0))
  (bind (_bblockinghit _binitialoverlap _time _distance _location_2 _impactpoint _normal) (`GameplayStatics.BreakHitResult` _outhit))
  (return _returnvalue (`KismetMathLibrary.MakeTransform` _impactpoint (`KismetMathLibrary.MakeRotFromZ` _normal))))

(fn `FindInstancesWithTransform`
  (params (InTransform :type "Transform Structure (by ref)") (HISM :type "HierarchicalInstancedStaticMeshComponent Object Reference"))
  (returns (IsSuccess :type Boolean) (Index :type Integer))
  (for _index (range (`InstancedStaticMeshComponent.GetInstanceCount` HISM))
    (if (== InTransform (`InstancedStaticMeshComponent.GetInstanceTransform` HISM _index true))
      (return true _index)))
  (return true 0))

(fn `get Color from Enum`
  (params (Instance :type Integer) (`Spawn Color` :type "/Game/fan_spawner/Miscs/Enums/EM_Spawn_Color Enum" :default "NewEnumerator0") (`Static Mesh` :type "InstancedStaticMeshComponent Object Reference") (WorldContextObject :type "Object Object Reference"))
  (returns (`To find instane with colour` :type Boolean) (`Liner Color Out` :type "LinearColor Structure") (OutputPin :type Integer))
  (locals (Material :type "MaterialInterface Object Reference"))
  (bind _returnvalue (== Instance (- (`InstancedStaticMeshComponent.GetInstanceCount` `Static Mesh`) 1)))
  (switch `/Game/fan_spawner/Miscs/Enums/EM_Spawn_Color` `Spawn Color`
    (:`NewEnumerator1`
      (set `local.Material` "/Game/fan_spawner/Materials/Chair_Color_Materials/M_Chair_black.M_Chair_black"))
    (:`NewEnumerator2`
      (set `local.Material` "/Game/fan_spawner/Materials/Chair_Color_Materials/M_Chair_dark_grey.M_Chair_dark_grey"))
    (:`NewEnumerator3`
      (set `local.Material` "/Game/fan_spawner/Materials/Chair_Color_Materials/M_Chair_light_grey.M_Chair_light_grey"))
    (:`NewEnumerator4`
      (set `local.Material` "/Game/fan_spawner/Materials/Chair_Color_Materials/M_Chair_White.M_Chair_White"))
    (:`NewEnumerator5`
      (set `local.Material` "/Game/fan_spawner/Materials/Chair_Color_Materials/M_Chair_Yellow.M_Chair_Yellow"))
    (:`NewEnumerator6`
      (set `local.Material` "/Game/fan_spawner/Materials/Chair_Color_Materials/M_Chair_Yellow_Orange.M_Chair_Yellow_Orange"))
    (:`NewEnumerator7`
      (set `local.Material` "/Game/fan_spawner/Materials/Chair_Color_Materials/M_Chair_Orange.M_Chair_Orange"))
    (:`NewEnumerator8`
      (set `local.Material` "/Game/fan_spawner/Materials/Chair_Color_Materials/M_Chair_Red_Orange.M_Chair_Red_Orange"))
    (:`NewEnumerator9`
      (set `local.Material` "/Game/fan_spawner/Materials/Chair_Color_Materials/M_Chair_Red.M_Chair_Red"))
    (:`NewEnumerator10`
      (set `local.Material` "/Game/fan_spawner/Materials/Chair_Color_Materials/M_Chair_Pink.M_Chair_Pink"))
    (:`NewEnumerator11`
      (set `local.Material` "/Game/fan_spawner/Materials/Chair_Color_Materials/M_Chair_Violet.M_Chair_Violet"))
    (:`NewEnumerator12`
      (set `local.Material` "/Game/fan_spawner/Materials/Chair_Color_Materials/M_Chair_Dark_Violet.M_Chair_Dark_Violet"))
    (:`NewEnumerator13`
      (set `local.Material` "/Game/fan_spawner/Materials/Chair_Color_Materials/M_Chair_blue.M_Chair_blue"))
    (:`NewEnumerator14`
      (set `local.Material` "/Game/fan_spawner/Materials/Chair_Color_Materials/M_Chair_Turquoise_Blue.M_Chair_Turquoise_Blue"))
    (:`NewEnumerator15`
      (set `local.Material` "/Game/fan_spawner/Materials/Chair_Color_Materials/M_Chair_Green.M_Chair_Green"))
    (:`NewEnumerator16`
      (set `local.Material` "/Game/fan_spawner/Materials/Chair_Color_Materials/M_Chair_Lime_Green.M_Chair_Lime_Green")))
  (bind _returnvalue_2 (`KismetMaterialLibrary.CreateDynamicMaterialInstance` WorldContextObject (`local.Material`) "None" "Transient"))
  (bind _returnvalue_3 (`MaterialInstanceDynamic.K2_GetVectorParameterValue` _returnvalue_2 "Param"))
  (bind (_r _g _b) (`KismetMathLibrary.BreakColor` _returnvalue_3))
  (`InstancedStaticMeshComponent.SetCustomDataValue` `Static Mesh` Instance 0 _r _returnvalue)
  (`InstancedStaticMeshComponent.SetCustomDataValue` `Static Mesh` Instance 1 _g _returnvalue)
  (bind _returnvalue_4 (`InstancedStaticMeshComponent.SetCustomDataValue` `Static Mesh` Instance 2 _b _returnvalue))
  (return _returnvalue_4 _returnvalue_3 Instance))

(fn `get material for widget`
  (params (`Spawn Color` :type "/Game/fan_spawner/Miscs/Enums/EM_Spawn_Color Enum" :default "NewEnumerator0") (WorldContextObject :type "Object Object Reference"))
  (returns (`Liner Color Out` :type "LinearColor Structure"))
  (locals (Material :type "MaterialInterface Object Reference"))
  (switch `/Game/fan_spawner/Miscs/Enums/EM_Spawn_Color` `Spawn Color`
    (:`NewEnumerator1`
      (set `local.Material` "/Game/fan_spawner/Materials/Chair_Color_Materials/M_Chair_black.M_Chair_black"))
    (:`NewEnumerator2`
      (set `local.Material` "/Game/fan_spawner/Materials/Chair_Color_Materials/M_Chair_dark_grey.M_Chair_dark_grey"))
    (:`NewEnumerator3`
      (set `local.Material` "/Game/fan_spawner/Materials/Chair_Color_Materials/M_Chair_light_grey.M_Chair_light_grey"))
    (:`NewEnumerator4`
      (set `local.Material` "/Game/fan_spawner/Materials/Chair_Color_Materials/M_Chair_White.M_Chair_White"))
    (:`NewEnumerator5`
      (set `local.Material` "/Game/fan_spawner/Materials/Chair_Color_Materials/M_Chair_Yellow.M_Chair_Yellow"))
    (:`NewEnumerator6`
      (set `local.Material` "/Game/fan_spawner/Materials/Chair_Color_Materials/M_Chair_Yellow_Orange.M_Chair_Yellow_Orange"))
    (:`NewEnumerator7`
      (set `local.Material` "/Game/fan_spawner/Materials/Chair_Color_Materials/M_Chair_Orange.M_Chair_Orange"))
    (:`NewEnumerator8`
      (set `local.Material` "/Game/fan_spawner/Materials/Chair_Color_Materials/M_Chair_Red_Orange.M_Chair_Red_Orange"))
    (:`NewEnumerator9`
      (set `local.Material` "/Game/fan_spawner/Materials/Chair_Color_Materials/M_Chair_Red.M_Chair_Red"))
    (:`NewEnumerator10`
      (set `local.Material` "/Game/fan_spawner/Materials/Chair_Color_Materials/M_Chair_Pink.M_Chair_Pink"))
    (:`NewEnumerator11`
      (set `local.Material` "/Game/fan_spawner/Materials/Chair_Color_Materials/M_Chair_Violet.M_Chair_Violet"))
    (:`NewEnumerator12`
      (set `local.Material` "/Game/fan_spawner/Materials/Chair_Color_Materials/M_Chair_Dark_Violet.M_Chair_Dark_Violet"))
    (:`NewEnumerator13`
      (set `local.Material` "/Game/fan_spawner/Materials/Chair_Color_Materials/M_Chair_blue.M_Chair_blue"))
    (:`NewEnumerator14`
      (set `local.Material` "/Game/fan_spawner/Materials/Chair_Color_Materials/M_Chair_Turquoise_Blue.M_Chair_Turquoise_Blue"))
    (:`NewEnumerator15`
      (set `local.Material` "/Game/fan_spawner/Materials/Chair_Color_Materials/M_Chair_Green.M_Chair_Green"))
    (:`NewEnumerator16`
      (set `local.Material` "/Game/fan_spawner/Materials/Chair_Color_Materials/M_Chair_Lime_Green.M_Chair_Lime_Green")))
  (bind _returnvalue (`KismetMaterialLibrary.CreateDynamicMaterialInstance` WorldContextObject (`local.Material`) "None" "Transient"))
  (bind _returnvalue_2 (`MaterialInstanceDynamic.K2_GetVectorParameterValue` _returnvalue "Param"))
  (bind (_r _g _b) (`KismetMathLibrary.BreakColor` _returnvalue_2))
  (return (`KismetMathLibrary.MakeColor` _r _g _b)))

(fn `GetGridSize`
  (params (LandscapeSize :type "Box2D Structure") (ItemCount :type Integer))
  (returns (ReturnValue :type Integer))
  (locals (Local_LandscapeSize :type "Box2D Structure"))
  (bind (_min _max) (break `Box2D` (`local.Local_LandscapeSize`)))
  (set `local.Local_LandscapeSize` LandscapeSize)
  (return (`KismetMathLibrary.FTrunc` (`KismetMathLibrary.Sqrt` (/ (* (`KismetMathLibrary.VSize2D` _min) (`KismetMathLibrary.VSize2D` _max)) (`KismetMathLibrary.Conv_IntToDouble` ItemCount))))))

(fn `GetInstanceLocationWithVariation`
  (params (BaseLocation :type "Vector Structure") (BaseLocationRightVector :type "Vector Structure") (BaseLocationUpVector :type "Vector Structure") (OffsetRight :type "Float (double-precision)") (OffsetRightVariation :type "Float (double-precision)") (OffsetUp :type "Float (double-precision)"))
  (returns (NewLocation :type "Vector Structure"))
  (bind _returnvalue (`KismetMathLibrary.Abs` OffsetRightVariation))
  (return (+ (`KismetMathLibrary.SelectVector` BaseLocation (+ BaseLocation (* BaseLocationRightVector (+ OffsetRight (`KismetMathLibrary.RandomFloatInRange` (* _returnvalue -1.0) _returnvalue)))) (and (== OffsetRight 0.0) (== OffsetRightVariation 0.0))) (`KismetMathLibrary.SelectVector` (0.0 0.0 0.0) (* BaseLocationUpVector OffsetUp) (== OffsetUp 0.0)))))

(fn `GetInstanceTransform`
  (params (ReferenceSpline :type "SplineComponent Object Reference") (SplinePointAtBaseLocation :type Integer :default -1) (SplineDistanceAtBaseLocation :type "Float (double-precision)") (SplinePointAtRotationTarget :type Integer :default -1) (SplineDistanceAtRotationTarget :type "Float (double-precision)") (UseBaseLocationAsRotationTarget :type Boolean) (OffsetRightFromRefSpline :type "Float (double-precision)") (OffsetUpFromRefSpline :type "Float (double-precision)") (OffsetRightVariation :type "Float (double-precision)") (RepeatOffset :type "Float (double-precision)") (MeshesAlwaysVertical :type Boolean) (__WorldContext1 :type "Object Object Reference"))
  (returns (NewTransform :type "Transform Structure"))
  (locals (BaseLocation :type "Vector Structure") (TargetLocation :type "Vector Structure") (BaseLocationRightVector :type "Vector Structure") (BaseLocationUpVector :type "Vector Structure") (BaseLocationTangent :type "Vector Structure") (MirrorFactor :type Integer) (L_UseBaseLocationAsRotTarget :type Boolean) (L_MirrorState :type Boolean) (L_MeshesAlwaysVertical :type Boolean) (L_RefSpline :type "SplineComponent Object Reference") (L_SplinePointAtBaseLocation :type Integer :default -1) (L_UseSplinePointAtBaseLocation :type Boolean) (L_SplineDistAtBaseLocation :type "Float (double-precision)") (L_SplinePointAtRotTarget :type Integer :default -1) (L_UseSplinePointAtRotTarget :type Boolean) (L_SplineDistAtRotTarget :type "Float (double-precision)") (L_OffsetRightFromRefSpline :type "Float (double-precision)") (L_OffsetUpFromRefSpline :type "Float (double-precision)") (L_RepeatOffset :type "Float (double-precision)") (L_OffsetRightVar :type "Float (double-precision)") (L_RotZ :type "Float (double-precision)") (L_RotZVar :type "Float (double-precision)") (L_BaseScale :type "Vector Structure") (L_BaseScaleVar :type "Float (double-precision)"))
  (bind _l_refspline (`local.L_RefSpline`))
  (bind _l_usesplinepointatbaselocation (`local.L_UseSplinePointAtBaseLocation`))
  (bind _l_splinepointatbaselocation (`local.L_SplinePointAtBaseLocation`))
  (bind _l_splinedistatbaselocation (`local.L_SplineDistAtBaseLocation`))
  (bind _returnvalue (`KismetMathLibrary.Conv_VectorToRotator` (`KismetMathLibrary.SelectVector` (`local.BaseLocationTangent`) (- (`local.TargetLocation`) (`local.BaseLocation`)) (`local.L_UseBaseLocationAsRotTarget`))))
  (set `local.L_RefSpline` ReferenceSpline)
  (bind _output_get (set `local.L_SplinePointAtBaseLocation` SplinePointAtBaseLocation))
  (set `local.L_UseSplinePointAtBaseLocation` (>= _output_get 0))
  (set `local.L_SplineDistAtBaseLocation` SplineDistanceAtBaseLocation)
  (bind _output_get_2 (set `local.L_SplinePointAtRotTarget` SplinePointAtRotationTarget))
  (set `local.L_UseSplinePointAtRotTarget` (>= _output_get_2 0))
  (set `local.L_SplineDistAtRotTarget` SplineDistanceAtRotationTarget)
  (set `local.L_UseBaseLocationAsRotTarget` UseBaseLocationAsRotationTarget)
  (set `local.L_OffsetRightFromRefSpline` OffsetRightFromRefSpline)
  (set `local.L_OffsetUpFromRefSpline` OffsetUpFromRefSpline)
  (set `local.L_OffsetRightVar` OffsetRightVariation)
  (set `local.L_RepeatOffset` RepeatOffset)
  (set `local.L_MeshesAlwaysVertical` MeshesAlwaysVertical)
  (`|ExecutionSequence`
    (:`then_0`
      (set `local.BaseLocation` (`KismetMathLibrary.SelectVector` (`SplineComponent.GetLocationAtSplinePoint` _l_refspline _l_splinepointatbaselocation "Local") (`SplineComponent.GetLocationAtDistanceAlongSpline` _l_refspline _l_splinedistatbaselocation "Local") _l_usesplinepointatbaselocation))
      (set `local.BaseLocationRightVector` (`KismetMathLibrary.SelectVector` (`SplineComponent.GetRightVectorAtSplinePoint` _l_refspline _l_splinepointatbaselocation "Local") (`SplineComponent.GetRightVectorAtDistanceAlongSpline` _l_refspline _l_splinedistatbaselocation "Local") _l_usesplinepointatbaselocation))
      (set `local.BaseLocationUpVector` (`KismetMathLibrary.SelectVector` (`SplineComponent.GetUpVectorAtSplinePoint` _l_refspline _l_splinepointatbaselocation "Local") (`SplineComponent.GetUpVectorAtDistanceAlongSpline` _l_refspline _l_splinedistatbaselocation "Local") _l_usesplinepointatbaselocation))
      (set `local.BaseLocationTangent` (`KismetMathLibrary.SelectVector` (`SplineComponent.GetTangentAtSplinePoint` _l_refspline _l_splinepointatbaselocation "Local") (`SplineComponent.GetTangentAtDistanceAlongSpline` _l_refspline _l_splinedistatbaselocation "Local") _l_usesplinepointatbaselocation))
      (set `local.TargetLocation` (`KismetMathLibrary.SelectVector` (`SplineComponent.GetLocationAtSplinePoint` _l_refspline (`local.L_SplinePointAtRotTarget`) "Local") (`SplineComponent.GetLocationAtDistanceAlongSpline` _l_refspline (`local.L_SplineDistAtRotTarget`) "Local") (`local.L_UseSplinePointAtRotTarget`))))
    (:`then_1`
      (return (`KismetMathLibrary.MakeTransform` (`self.GetInstanceLocationWithVariation` (`local.BaseLocation`) (`local.BaseLocationRightVector`) (`local.BaseLocationUpVector`) (+ (`local.L_RepeatOffset`) (`local.L_OffsetRightFromRefSpline`)) (`local.L_OffsetRightVar`) (`local.L_OffsetUpFromRefSpline`) __WorldContext1) (`KismetMathLibrary.SelectRotator` (`KismetMathLibrary.MakeRotator` 0.0 0.0 (.yaw _returnvalue)) _returnvalue (`local.L_MeshesAlwaysVertical`)))))))

(fn `IsEvenNumber`
  (params (Number :type Integer))
  (returns (IsEven :type Boolean))
  (bind _returnvalue (/ (`KismetMathLibrary.Conv_IntToDouble` Number) 2.0))
  (return (== (- _returnvalue (`KismetMathLibrary.Conv_IntToDouble` (`KismetMathLibrary.FTrunc` _returnvalue))) 0.0)))

(fn `IsPointIntoSpline`
  (params (PointLocation :type "Vector2D Structure") (Spline :type "SplineComponent Object Reference") (LandcapeSize :type "Box2D Structure (by ref)"))
  (returns (ReturnValue :type Boolean))
  (locals (Local_PointLocation :type "Vector2D Structure") (Local_IntersectionNumber :type Integer) (Local_LanscapeSize :type "Box2D Structure") (Local_Spline :type "SplineComponent Object Reference"))
  (bind _local_pointlocation (`local.Local_PointLocation`))
  (bind _returnvalue (`SplineComponent.GetNumberOfSplinePoints` (`local.Local_Spline`)))
  (set `local.Local_PointLocation` PointLocation)
  (set `local.Local_Spline` Spline)
  (set `local.Local_LanscapeSize` LandcapeSize)
  (for _index (range _returnvalue)
    (bind _returnvalue_2 (+ _index 1))
    (bind _returnvalue_3 (`self.IsTwoSegmentsIntersect` (`KismetMathLibrary.MakeBox2D` (`KismetMathLibrary.MakeVector2D` (.x (`SplineComponent.GetLocationAtSplinePoint` (`local.Local_Spline`) (select `bool` (> _returnvalue_2 (- _returnvalue 0)) :`false` _returnvalue_2) "World")) (.y (`SplineComponent.GetLocationAtSplinePoint` (`local.Local_Spline`) (select `bool` (> _returnvalue_2 (- _returnvalue 0)) :`false` _returnvalue_2) "World"))) (`KismetMathLibrary.MakeVector2D` (.x (`SplineComponent.GetLocationAtSplinePoint` (`local.Local_Spline`) _index "World")) (.y (`SplineComponent.GetLocationAtSplinePoint` (`local.Local_Spline`) _index "World")))) (`KismetMathLibrary.MakeBox2D` (+ _local_pointlocation (`self.Vector2Vector2d` (* (`SceneComponent.GetForwardVector` (`local.Local_Spline`)) 500000.0))) _local_pointlocation) Spline))
    (if _returnvalue_3
      (`/Engine/EditorBlueprintResources/StandardMacros.IncrementInt` (`local.Local_IntersectionNumber`))))
  (return (not (`self.IsEvenNumber` (`local.Local_IntersectionNumber`)))))

(fn `IsTwoSegmentsIntersect`
  (params (Segment1 :type "Box2D Structure") (Segment2 :type "Box2D Structure"))
  (returns (ReturnValue :type Boolean))
  (locals (L_A :type "Vector2D Structure") (L_B :type "Vector2D Structure") (L_C :type "Vector2D Structure") (L_D :type "Vector2D Structure") (X :type "Float (double-precision)") (Y :type "Float (double-precision)"))
  (bind (_min _max) (break `Box2D` Segment1))
  (bind (_min_2 _max_2) (break `Box2D` Segment2))
  (bind _x (`KismetMathLibrary.BreakVector2D` (`local.L_C`)))
  (bind _x_2 (`KismetMathLibrary.BreakVector2D` (`local.L_D`)))
  (bind (_x_3 _y) (`KismetMathLibrary.BreakVector2D` (`local.L_C`)))
  (bind (_x_4 _y_2) (`KismetMathLibrary.BreakVector2D` (`local.L_D`)))
  (bind (_x_5 _y_3) (`KismetMathLibrary.BreakVector2D` (`local.L_A`)))
  (bind (_x_6 _y_4) (`KismetMathLibrary.BreakVector2D` (`local.L_B`)))
  (bind (_x_7 _y_5) (`KismetMathLibrary.BreakVector2D` (`local.L_C`)))
  (bind (_x_8 _y_6) (`KismetMathLibrary.BreakVector2D` (`local.L_D`)))
  (bind _x_9 (`KismetMathLibrary.BreakVector2D` (`local.L_A`)))
  (bind _x_10 (`KismetMathLibrary.BreakVector2D` (`local.L_B`)))
  (bind _returnvalue (- _x_4 _x_3))
  (bind _returnvalue_2 (- (* (- _y _y_2) (`local.X`)) (- (* _x_3 _y_2) (* _x_4 _y))))
  (bind _returnvalue_3 (- (* (- _y_3 _y_4) (- _x_8 _x_7)) (* (- _y_5 _y_6) (- _x_6 _x_5))))
  (bind _returnvalue_4 (- (* (- (* _x_5 _y_4) (* _x_6 _y_3)) (- _x_8 _x_7)) (* (- (* _x_7 _y_6) (* _x_8 _y_5)) (- _x_6 _x_5))))
  (set `local.L_A` _min)
  (set `local.L_B` _max)
  (set `local.L_C` _min_2)
  (set `local.L_D` _max_2)
  (if (or (== _returnvalue_4 0.0) (== _returnvalue_3 0.0) (== _returnvalue_2 0.0) (== _returnvalue 0.0))
    (return false)
    (else
      (set `local.X` (* (/ _returnvalue_4 _returnvalue_3) -1.0))
      (set `local.Y` (/ _returnvalue_2 _returnvalue))
      (return (and (or (and (<= _x (`local.X`)) (>= _x_2 (`local.X`))) (and (<= _x_2 (`local.X`)) (>= _x (`local.X`)))) (or (and (<= _x_9 (`local.X`)) (>= _x_10 (`local.X`))) (and (<= _x_10 (`local.X`)) (>= _x_9 (`local.X`)))))))))

(fn `rotation`
  (params (`Actor rotation and location` :type "Actor Object Reference") (Distance :type "Float (double-precision)"))
  (returns (`out point` :type "Vector Structure"))
  (return (+ (`Actor.K2_GetActorLocation` `Actor rotation and location`) (* (`KismetMathLibrary.GetForwardVector` (`Actor.K2_GetActorRotation` `Actor rotation and location`)) Distance))))

(fn `set instance color`
  (params (Instance :type Integer) (`Static Mesh` :type "InstancedStaticMeshComponent Object Reference") (bMarkRenderStateDirty :type Boolean) (InColor :type "LinearColor Structure"))
  (returns (`To find instane with colour` :type Boolean) (` Out Color` :type "LinearColor Structure"))
  (bind (_r _g _b) (`KismetMathLibrary.BreakColor` InColor))
  (`InstancedStaticMeshComponent.SetCustomDataValue` `Static Mesh` Instance 0 _r bMarkRenderStateDirty)
  (`InstancedStaticMeshComponent.SetCustomDataValue` `Static Mesh` Instance 1 _g bMarkRenderStateDirty)
  (bind _returnvalue (`InstancedStaticMeshComponent.SetCustomDataValue` `Static Mesh` Instance 2 _b bMarkRenderStateDirty))
  (return _returnvalue InColor))

(fn `Square Transform`
  (params (BP_AutoSpawner :type "/Game/fan_spawner/Blueprints/Main_Blueprints/BP_Fan_Spawner Object Reference") (`chair rot` :type "Float (double-precision)") (`row distance` :type "Float (double-precision)") (`colum dis ` :type "Float (double-precision)"))
  (returns (`chair transforms` :type "Array of Transform Structure"))
  (locals (Local_LandscapeSize :type "Box2D Structure") (Local_Spline :type "SplineComponent Object Reference") (`row dis` :type "Float (double-precision)") (Local_GridSize :type Integer) (Local_chair_transfrom :type "Array of Transform Structure") (Local_BP_AutoSPawner :type "/Game/fan_spawner/Blueprints/Main_Blueprints/BP_Fan_Spawner Object Reference") (`colum dis` :type "Float (double-precision)") (`chair height` :type "Float (double-precision)") (Local_fans_transfrom :type "Array of Transform Structure"))
  (bind _returnvalue (`Actor.K2_GetActorRotation` (`local.Local_BP_AutoSPawner`)))
  (bind (_x _y) (`KismetMathLibrary.BreakVector2D` (/ (`.Max` (break `Box2D` (`local.Local_LandscapeSize`))) (`local.colum dis`))))
  (bind (_x_2 _y_2) (`KismetMathLibrary.BreakVector2D` (/ (`.Min` (break `Box2D` (`local.Local_LandscapeSize`))) (`local.row dis`))))
  (bind _output_get (set `local.Local_BP_AutoSPawner` BP_AutoSpawner))
  (set `local.Local_LandscapeSize` (`/Game/fan_spawner/Blueprints/Main_Blueprints/BP_Fan_Spawner.LandscapeSize` _output_get))
  (set `local.Local_Spline` (`/Game/fan_spawner/Blueprints/Main_Blueprints/BP_Fan_Spawner.Spline` _output_get))
  (set `local.row dis` `row distance`)
  (set `local.colum dis` `colum dis `)
  (set `local.chair height` (`/Game/fan_spawner/Blueprints/Main_Blueprints/BP_Fan_Spawner.chairs height` _output_get))
  (`|ExecutionSequence`
    (:`then_0`
      (for _index (range (`KismetMathLibrary.FTrunc` _x_2) (+ (`KismetMathLibrary.FTrunc` _y_2) 1)) :!pinned true
        ;[1 1 1] get rotation at world locations
        (for _index_2 (range (`KismetMathLibrary.FTrunc` _x) (+ (`KismetMathLibrary.FTrunc` _y) 1))
          (bind _returnvalue_2 (`KismetMathLibrary.RotateAngleAxis` (`KismetMathLibrary.MakeVector` (* _index (`local.row dis`)) (* _index_2 (`local.colum dis`)) (* _index (`local.chair height`))) (.yaw _returnvalue) (0.0 0.0 1.0)))
          (bind _returnvalue_3 (`self.IsPointIntoSpline` (`self.Vector2Vector2d` (+ (`Actor.K2_GetActorLocation` (`local.Local_BP_AutoSPawner`)) _returnvalue_2)) (`local.Local_Spline`) (`local.Local_LandscapeSize`))) ; Does the point lie in the polygon
          (if _returnvalue_3
            (`KismetArrayLibrary.Array_Add` (`local.Local_chair_transfrom`) (`KismetMathLibrary.MakeTransform` _returnvalue_2 _returnvalue))))))
    (:`then_1`
      (return (`local.Local_chair_transfrom`)))))

(fn `ValidateStartAndEndPoints`
  (params (`Base Spline` :type "SplineComponent Object Reference"))
  (returns (ValidatedEndPoint :type Integer))
  (return (- (`SplineComponent.GetNumberOfSplinePoints` `Base Spline`) 1)))

(fn `Vector2d2Vector`
  (params (Vector2d :type "Vector2D Structure") (Z :type "Float (double-precision)"))
  (returns (ReturnValue :type "Vector Structure"))
  (bind (_x _y) (`KismetMathLibrary.BreakVector2D` Vector2d))
  (return (`KismetMathLibrary.MakeVector` _x _y Z)))

(fn `Vector2Vector2d`
  (params (Vector :type "Vector Structure"))
  (returns (ReturnValue :type "Vector2D Structure") (Z :type "Float (double-precision)"))
  (return (`KismetMathLibrary.MakeVector2D` (.x Vector) (.y Vector)) (.z Vector)))