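; BP_Phone_Light is a short-lived point light actor that flickers and then removes itself, named as a phone light.
; The construction script applies the LightColor variable to the point light.
; On BeginPlay it toggles the light's visibility, waits a second, runs a rapid burst of further toggles through chained delays, then destroys the actor.
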(event `self.ReceiveBeginPlay`
  (bind _pointlight (`self.PointLight`))
  (`SceneComponent.ToggleVisibility` _pointlight false)
  (`KismetSystemLibrary.Delay` 1.0)
  (`SceneComponent.ToggleVisibility` _pointlight false)
  (`KismetSystemLibrary.Delay` 0.1)
  (`SceneComponent.ToggleVisibility` _pointlight false)
  (`KismetSystemLibrary.Delay` 0.1)
  (`SceneComponent.ToggleVisibility` _pointlight false)
  (`KismetSystemLibrary.Delay` 0.1)
  (`SceneComponent.ToggleVisibility` _pointlight false)
  (`KismetSystemLibrary.Delay` 0.1)
  (`SceneComponent.ToggleVisibility` _pointlight false)
  (`KismetSystemLibrary.Delay` 0.1)
  (`self.K2_DestroyActor`))

(fn `UserConstructionScript`
  (`LightComponent.SetLightColor` (`self.PointLight`) (`self.Light_Color`) true))