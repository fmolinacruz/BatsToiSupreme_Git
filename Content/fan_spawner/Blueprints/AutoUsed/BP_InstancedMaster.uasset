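; Helper actor that turns a BP_AutoSpawner's settings into instanced crowd seating on a BP_fans actor, then destroys itself.
; A chair data table row supplies mesh, spacing and offsets for either a square layout or spline rows, built from offset copies of the base spline with mitred corners.
; Each transform, optionally ground-adjusted, becomes a colored chair or standing-placeholder instance on a new or existing BP_fans, which then gathers fan locations.
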(fn `AddInstanced`
  (params (SpawnItem :type "/Game/fan_spawner/Structs/ST_SpawnItemInformation Structure (by ref)") (BP_AutoSpawner :type "/Game/fan_spawner/Blueprints/Main_Blueprints/BP_Fan_Spawner Object Reference"))
  (bind _returnvalue (`|SpawnActorFromClass` "/Game/fan_spawner/Blueprints/AutoUsed/BP_fans.BP_fans_C" (`KismetMathLibrary.MakeTransform` (`self.to spawn fan bp`)) "AlwaysSpawn" "OverrideRootScale" null self BP_AutoSpawner null))
  (set `self.fan bp` _returnvalue)
  (bind _chair_model (`/Game/fan_spawner/Blueprints/AutoUsed/BP_fans.chair model` _returnvalue))
  (`PrimitiveComponent.SetCollisionObjectType` _chair_model "ECC_WorldStatic")
  (`PrimitiveComponent.SetCollisionResponseToChannel` _chair_model "ECC_WorldStatic" "ECR_Ignore")
  (`StaticMeshComponent.SetStaticMesh` _chair_model (`.StaticMesh_30_522DE65D4966FD875D3ACBB74082D926` (break `/Game/fan_spawner/Structs/ST_SpawnItemInformation` SpawnItem))))

(fn `GetInstanceRotWithVariation`
  (params (BaseRotation :type "Rotator Structure") (MeshRotZ :type "Float (double-precision)") (MeshRotZVariation :type "Float (double-precision)"))
  (returns (NewRotation :type "Rotator Structure"))
  (locals (L_RotZWithVar :type "Float (double-precision)"))
  (bind _returnvalue (`KismetMathLibrary.Abs` MeshRotZVariation))
  (bind _output_get (set `local.L_RotZWithVar` (+ (`KismetMathLibrary.SelectFloat` 0.0 (`KismetMathLibrary.RandomFloatInRange` (* _returnvalue -1.0) _returnvalue) (== MeshRotZVariation 0.0)) MeshRotZ)))
  (return (`KismetMathLibrary.ComposeRotators` BaseRotation (`KismetMathLibrary.RotatorFromAxisAndAngle` (`KismetMathLibrary.GetUpVector` BaseRotation) _output_get))))

(fn `Line Transform`
  (params (`Auto Spawner Ref` :type "/Game/fan_spawner/Blueprints/Main_Blueprints/BP_Fan_Spawner Object Reference") (Rows :type "Float (double-precision)") (Collum :type "Float (double-precision)"))
  (returns (`Chair Transform` :type "Array of Transform Structure"))
  (locals (`bp auto spawnner` :type "/Game/fan_spawner/Blueprints/Main_Blueprints/BP_Fan_Spawner Object Reference") (`Chairs Array` :type "Array of Transform Structure") (`row of chairs` :type Integer))
  (bind _returnvalue (`self.K2_GetActorRotation` `Auto Spawner Ref`))
  (bind _returnvalue_2 (`KismetMathLibrary.Conv_IntToDouble` (`local.row of chairs`)))
  (bind _returnvalue_3 (`KismetMathLibrary.Conv_IntToDouble` (`local.row of chairs`)))
  (for _index (range (`/Game/fan_spawner/Blueprints/Main_Blueprints/BP_Fan_Spawner.Num of Chairs Going Back` `Auto Spawner Ref`))
    (set `local.row of chairs` _index)
    (bind _output_get (set `local.bp auto spawnner` `Auto Spawner Ref`))
    (bind _newoffsetsplinedetails (`self.OffsetASpline` _output_get (* _returnvalue_3 Rows) (* _returnvalue_3 (`/Game/fan_spawner/Blueprints/Main_Blueprints/BP_Fan_Spawner.chairs height` `Auto Spawner Ref`)) (* Collum (`/Game/fan_spawner/Blueprints/Main_Blueprints/BP_Fan_Spawner.curve smoothness ` `Auto Spawner Ref`))))
    (bind _output_get_2 (set `self.PointElemOffsetSplines` _newoffsetsplinedetails))
    (bind _instancetransforms (`/Game/fan_spawner/Blueprints/AutoUsed/BP_AutoSpawnerLibrary.Calculate Point Transforms` _output_get_2 (* _returnvalue_2 Rows) (* _returnvalue_2 (`/Game/fan_spawner/Blueprints/Main_Blueprints/BP_Fan_Spawner.chairs height` `Auto Spawner Ref`)) Collum (`/Game/fan_spawner/Blueprints/Main_Blueprints/BP_Fan_Spawner.Base Spline ` (`local.bp auto spawnner`)) self))
    (for _array_element _instancetransforms
      (`KismetArrayLibrary.Array_Add` (`local.Chairs Array`) (`KismetMathLibrary.MakeTransform` (`KismetMathLibrary.RotateAngleAxis` (+ (.location (`self.offset Transform`)) (.location _array_element)) (.yaw _returnvalue) (0.0 0.0 1.0)) (`KismetMathLibrary.MakeRotator` 0.0 0.0 (+ (.yaw (.rotation _array_element)) (.yaw _returnvalue) 90.0 (.yaw (.rotation (`self.offset Transform`)))))))))
  (return (`local.Chairs Array`)))

(fn `OffsetASpline`
  (params (`Auto Spawner Ref` :type "/Game/fan_spawner/Blueprints/Main_Blueprints/BP_Fan_Spawner Object Reference") (OffsetRight :type "Float (double-precision)") (OffsetUp :type "Float (double-precision)") (Spacing :type "Float (double-precision)"))
  (returns (NewOffsetSplineDetails :type "/Game/fan_spawner/Structs/ST_OffsetSpline Structure"))
  (locals (L_OffsetRight :type "Float (double-precision)") (L_ForcedVerticalAxis :type Boolean) (L_SplineStartPointIndex :type Integer) (L_SplineEndPointIndex :type Integer) (L_CurrentPointIndex :type Integer) (L_CurrentPointType :type "ESplinePointType Enum") (L_OffsetSpline :type "SplineComponent Object Reference") (OffsetSplineDrawDebug :type Boolean) (L_DistanceAtBasePoint :type "Array of Float (double-precision)") (L_IsCornerPoint :type "Array of Boolean") (L_IsFirstLoop :type Boolean) (L_EndDistance :type "Float (double-precision)") (L_CurrentDistance :type "Float (double-precision)") (L_IsUsingBaseSplineAsOffsetSpline :type Boolean) (L_Spacing :type "Float (double-precision)") (`L_Offset Up` :type "Float (double-precision)") (`L base Spline` :type "SplineComponent Object Reference"))
  (bind _l_base_spline (`local.L base Spline`))
  (bind _l_currentpointindex (`local.L_CurrentPointIndex`))
  (bind _l_currentpointindex_2 (`local.L_CurrentPointIndex`))
  (bind _l_base_spline_2 (`local.L base Spline`))
  (bind _l_base_spline_3 (`local.L base Spline`))
  (bind _l_currentpointindex_3 (`local.L_CurrentPointIndex`))
  (bind _l_base_spline_4 (`local.L base Spline`))
  (bind _l_base_spline_5 (`local.L base Spline`))
  (bind _l_base_spline_6 (`local.L base Spline`))
  (bind _l_currentpointindex_4 (`local.L_CurrentPointIndex`))
  (bind _l_offsetspline (`local.L_OffsetSpline`))
  (bind _l_forcedverticalaxis (`local.L_ForcedVerticalAxis`))
  (bind _l_offsetspline_2 (`local.L_OffsetSpline`))
  (bind _l_forcedverticalaxis_2 (`local.L_ForcedVerticalAxis`))
  (bind _l_currentpointindex_5 (`local.L_CurrentPointIndex`))
  (bind _l_base_spline_7 (`local.L base Spline`))
  (bind _l_base_spline_8 (`local.L base Spline`))
  (bind _l_currentdistance (`local.L_CurrentDistance`))
  (bind _l_offsetspline_3 (`local.L_OffsetSpline`))
  (bind _l_splineendpointindex (`local.L_SplineEndPointIndex`))
  (bind _l_splineendpointindex_2 (`local.L_SplineEndPointIndex`))
  (bind _l_splineendpointindex_3 (`local.L_SplineEndPointIndex`))
  (bind _l_base_spline_9 (`local.L base Spline`))
  (bind _l_splineendpointindex_4 (`local.L_SplineEndPointIndex`))
  (bind _l_offsetspline_4 (`local.L_OffsetSpline`))
  (bind _l_offsetspline_5 (`local.L_OffsetSpline`))
  (bind _l_offsetspline_6 (`local.L_OffsetSpline`))
  (bind _l_iscornerpoint (`local.L_IsCornerPoint`))
  (bind _l_offset_up (`local.L_Offset Up`))
  (bind _l_offset_up_2 (`local.L_Offset Up`))
  (bind _l_offset_up_3 (`local.L_Offset Up`))
  (bind _l_offset_up_4 (`local.L_Offset Up`))
  (bind _l_offset_up_5 (`local.L_Offset Up`))
  (bind _returnvalue (`SplineComponent.GetUpVectorAtSplinePoint` _l_base_spline_8 _l_currentpointindex_2 "Local"))
  (bind _returnvalue_2 (`SplineComponent.GetUpVectorAtSplinePoint` _l_base_spline _l_splineendpointindex_4 "Local"))
  (bind _returnvalue_3 (- (`SplineComponent.GetDistanceAlongSplineAtSplinePoint` _l_base_spline_9 _l_splineendpointindex_3) 0.01))
  (bind _returnvalue_4 (- (`SplineComponent.GetNumberOfSplinePoints` _l_offsetspline_6) 1))
  (bind _returnvalue_5 (- (`SplineComponent.GetNumberOfSplinePoints` _l_offsetspline) 1))
  (bind _returnvalue_6 (- (`SplineComponent.GetNumberOfSplinePoints` _l_offsetspline_2) 1))
  (bind _returnvalue_7 (- (`SplineComponent.GetNumberOfSplinePoints` _l_offsetspline_4) 1))
  (bind _returnvalue_8 (/ (- (`KismetMathLibrary.Vector_HeadingAngle` (`SplineComponent.GetDirectionAtDistanceAlongSpline` _l_base_spline_3 (- (`SplineComponent.GetDistanceAlongSplineAtSplinePoint` _l_base_spline_3 _l_splineendpointindex_2) 0.01) "Local")) (`KismetMathLibrary.Vector_HeadingAngle` (`SplineComponent.GetDirectionAtSplinePoint` _l_base_spline_3 _l_splineendpointindex_2 "Local"))) 2.0))
  (bind _returnvalue_9 (/ (- (`KismetMathLibrary.Vector_HeadingAngle` (`SplineComponent.GetDirectionAtDistanceAlongSpline` _l_base_spline_7 (- (`SplineComponent.GetDistanceAlongSplineAtSplinePoint` _l_base_spline_7 _l_currentpointindex_4) 0.01) "Local")) (`KismetMathLibrary.Vector_HeadingAngle` (`SplineComponent.GetDirectionAtSplinePoint` _l_base_spline_7 _l_currentpointindex_4 "Local"))) 2.0))
  ;[1 1 1] Only proceed creating the offset spline if Spacing is > 0 (as no mesh will be generated if spacing is 0)
  (bind _output_get (set `local.L_Spacing` Spacing))
  (if (> _output_get 0.0)
    (set `local.L_OffsetRight` OffsetRight)
    (set `local.L_Offset Up` OffsetUp)
    (set `local.L_ForcedVerticalAxis` false)
    (set `local.L base Spline` (`/Game/fan_spawner/Blueprints/Main_Blueprints/BP_Fan_Spawner.Base Spline ` `Auto Spawner Ref`))
    (set `local.L_SplineStartPointIndex` 0)
    (set `local.L_SplineEndPointIndex` (`/Game/fan_spawner/Blueprints/AutoUsed/BP_AutoSpawnerLibrary.ValidateStartAndEndPoints` (`local.L base Spline`)))
    (`KismetArrayLibrary.Array_Clear` (`local.L_IsCornerPoint`))
    (`KismetArrayLibrary.Array_Clear` (`local.L_DistanceAtBasePoint`))
    (`|ExecutionSequence`
      (:`then_0`
        ;[1 1 1] If there's no offset, then a simplier method will be used to generate the OffsetSpline to save performance when regenerating the meshes
        (bind _output_get_2 (set `local.L_IsUsingBaseSplineAsOffsetSpline` (and (== (`local.L_OffsetRight`) 0.0) (== (`local.L_Offset Up`) 0.0))))
        (if _output_get_2
          ;[0.4317 1 0.3906] OffsetRight and OffsetUp are both 0 - OffsetSpline is not required, BaseSpline will be referenced instead
          (set `local.L_OffsetSpline` (`local.L base Spline`))
          (for _index (range (`local.L_SplineStartPointIndex`) (+ (`local.L_SplineEndPointIndex`) 1))
            (`KismetArrayLibrary.Array_Add` (`local.L_DistanceAtBasePoint`) (`SplineComponent.GetDistanceAlongSplineAtSplinePoint` _l_offsetspline_5 _index))
            (if (== _index (`local.L_SplineStartPointIndex`))
              (`KismetArrayLibrary.Array_Add` _l_iscornerpoint)
              (else
                (`KismetArrayLibrary.Array_Add` _l_iscornerpoint (and (`|EnumEquality` (`SplineComponent.GetSplinePointType` _l_offsetspline_5 _index) "Linear") (`|EnumEquality` (`SplineComponent.GetSplinePointType` _l_offsetspline_5 (+ _index -1)) "Linear"))))))
          (else
            (bind _returnvalue_10 (`AddComponent|NODE_AddSplineComponent-0`))
            (bind _output_get_3 (set `local.L_OffsetSpline` _returnvalue_10))
            (set `SplineComponent.bDrawDebug` (`local.OffsetSplineDrawDebug`) _returnvalue_10)
            (`SplineComponent.ClearSplinePoints` _output_get_3 true)
            (for _index_2 (range (`local.L_SplineStartPointIndex`) (`local.L_SplineEndPointIndex`))
              (bind _output_get_4 (set `local.L_CurrentPointIndex` _index_2))
              (bind _output_get_5 (set `local.L_CurrentPointType` (`SplineComponent.GetSplinePointType` (`local.L base Spline`) _output_get_4)))
              (if (`|EnumEquality` _output_get_5 "Linear")
                (if (and (> _l_currentpointindex_3 0) (< _l_currentpointindex_3 (- (`SplineComponent.GetNumberOfSplinePoints` (`local.L base Spline`)) 1)))
                  (if (`|EnumEquality` (`SplineComponent.GetSplinePointType` (`local.L base Spline`) (- (`local.L_CurrentPointIndex`) 1)) "Linear")
                    ;[1 1 1] When the current and last point type are both linear - i.e. a Corner Point. Use math to calculate offset point location
                    (`SplineComponent.AddSplinePoint` _l_offsetspline_2 (+ (`SplineComponent.GetLocationAtSplinePoint` _l_base_spline_8 _l_currentpointindex_2 "Local") (* (`KismetMathLibrary.RotateAngleAxis` (`SplineComponent.GetRightVectorAtSplinePoint` _l_base_spline_8 _l_currentpointindex_2 "Local") (`KismetMathLibrary.RadiansToDegrees` _returnvalue_9) (`KismetMathLibrary.SelectVector` (0.0 0.0 1.0) _returnvalue _l_forcedverticalaxis)) (/ (`local.L_OffsetRight`) (`KismetMathLibrary.Cos` (`KismetMathLibrary.Abs` _returnvalue_9)))) (`KismetMathLibrary.SelectVector` (`KismetMathLibrary.MakeVector` 0.0 0.0 _l_offset_up_4) (* _returnvalue _l_offset_up_4) _l_forcedverticalaxis)) "Local" true)
                    (`SplineComponent.SetSplinePointType` _l_offsetspline_2 _returnvalue_6 "Linear" true)
                    (`KismetArrayLibrary.Array_Add` (`local.L_DistanceAtBasePoint`) (`SplineComponent.GetDistanceAlongSplineAtSplinePoint` _l_offsetspline_2 _returnvalue_6))
                    (`KismetArrayLibrary.Array_Add` (`local.L_IsCornerPoint`) true)
                    (else
                      ;[1 1 1] For any other linear points - get offset location based on spline point axis
                      (`SplineComponent.AddSplinePoint` _l_offsetspline_6 (+ (`SplineComponent.GetLocationAtSplinePoint` _l_base_spline_6 _l_currentpointindex_5 "Local") (* (`SplineComponent.GetRightVectorAtSplinePoint` _l_base_spline_6 _l_currentpointindex_5 "Local") (`local.L_OffsetRight`)) (`KismetMathLibrary.SelectVector` (`KismetMathLibrary.MakeVector` 0.0 0.0 _l_offset_up_5) (* (`SplineComponent.GetUpVectorAtSplinePoint` _l_base_spline_6 _l_currentpointindex_5 "Local") _l_offset_up_5) (`local.L_ForcedVerticalAxis`))) "Local" true :!label _label)
                      (`SplineComponent.SetTangentAtSplinePoint` _l_offsetspline_6 _returnvalue_4 (`SplineComponent.GetTangentAtSplinePoint` _l_base_spline_6 _l_currentpointindex_5 "Local") "Local" false)
                      (`SplineComponent.SetSplinePointType` _l_offsetspline_6 _returnvalue_4 "Linear" true)
                      (`KismetArrayLibrary.Array_Add` (`local.L_DistanceAtBasePoint`) (`SplineComponent.GetDistanceAlongSplineAtSplinePoint` _l_offsetspline_6 _returnvalue_4))
                      (`KismetArrayLibrary.Array_Add` (`local.L_IsCornerPoint`))))
                  (else
                    (goto _label)))
                (else
                  ;[1 1 1] For any non-linear points - While Loop is used to generate a point every spacing/2
                  (set `local.L_CurrentDistance` (`SplineComponent.GetDistanceAlongSplineAtSplinePoint` _l_base_spline_4 _l_currentpointindex))
                  (set `local.L_EndDistance` (`SplineComponent.GetDistanceAlongSplineAtSplinePoint` _l_base_spline_4 (+ _l_currentpointindex 1)))
                  (set `local.L_IsFirstLoop` true)
                  (while (< (`local.L_CurrentDistance`) (`local.L_EndDistance`))
                    (`SplineComponent.AddSplinePoint` _l_offsetspline_4 (+ (`SplineComponent.GetLocationAtDistanceAlongSpline` _l_base_spline_5 _l_currentdistance "Local") (* (`SplineComponent.GetRightVectorAtDistanceAlongSpline` _l_base_spline_5 _l_currentdistance "Local") (`local.L_OffsetRight`)) (`KismetMathLibrary.SelectVector` (`KismetMathLibrary.MakeVector` 0.0 0.0 _l_offset_up_3) (* (`SplineComponent.GetUpVectorAtDistanceAlongSpline` _l_base_spline_5 _l_currentdistance "Local") _l_offset_up_3) (`local.L_ForcedVerticalAxis`))) "Local" true)
                    (`SplineComponent.SetTangentAtSplinePoint` _l_offsetspline_4 _returnvalue_7 (`SplineComponent.GetTangentAtDistanceAlongSpline` _l_base_spline_5 _l_currentdistance "Local") "Local" false)
                    (`SplineComponent.SetSplinePointType` _l_offsetspline_4 _returnvalue_7 "Linear" true)
                    (if (`local.L_IsFirstLoop`)
                      (`KismetArrayLibrary.Array_Add` (`local.L_DistanceAtBasePoint`) (`SplineComponent.GetDistanceAlongSplineAtSplinePoint` _l_offsetspline_4 _returnvalue_7))
                      (`KismetArrayLibrary.Array_Add` (`local.L_IsCornerPoint`))
                      (set `local.L_IsFirstLoop` false))
                    ;;[1 0.2141 0] IMPORTAMNT - this is needed to progress the While Loop. Disconnecting this will result in infinite loop
                    (set `local.L_CurrentDistance` (+ (`local.L_CurrentDistance`) (`local.L_Spacing`)))))))
            ;[1 1 1] Offset the last point
            (if (and (`|EnumEquality` (`SplineComponent.GetSplinePointType` _l_base_spline_2 _l_splineendpointindex) "Linear") (`|EnumEquality` (`SplineComponent.GetSplinePointType` _l_base_spline_2 (- _l_splineendpointindex 1)) "Linear"))
              (`SplineComponent.AddSplinePoint` _l_offsetspline (+ (`SplineComponent.GetLocationAtSplinePoint` _l_base_spline _l_splineendpointindex_4 "Local") (* (`KismetMathLibrary.RotateAngleAxis` (`SplineComponent.GetRightVectorAtSplinePoint` _l_base_spline _l_splineendpointindex_4 "Local") (`KismetMathLibrary.RadiansToDegrees` _returnvalue_8) (`KismetMathLibrary.SelectVector` (0.0 0.0 1.0) _returnvalue_2 _l_forcedverticalaxis_2)) (/ (`local.L_OffsetRight`) (`KismetMathLibrary.Cos` (`KismetMathLibrary.Abs` _returnvalue_8)))) (`KismetMathLibrary.SelectVector` (`KismetMathLibrary.MakeVector` 0.0 0.0 _l_offset_up_2) (* _returnvalue_2 _l_offset_up_2) _l_forcedverticalaxis_2)) "Local" true)
              (else
                (`SplineComponent.AddSplinePoint` _l_offsetspline_3 (+ (`SplineComponent.GetLocationAtSplinePoint` _l_base_spline_9 _l_splineendpointindex_3 "Local") (* (`SplineComponent.GetRightVectorAtDistanceAlongSpline` _l_base_spline_9 _returnvalue_3 "Local") (`local.L_OffsetRight`)) (`KismetMathLibrary.SelectVector` (`KismetMathLibrary.MakeVector` 0.0 0.0 _l_offset_up) (* (`SplineComponent.GetUpVectorAtDistanceAlongSpline` _l_base_spline_9 _returnvalue_3 "Local") _l_offset_up) (`local.L_ForcedVerticalAxis`))) "Local" true)
                (`SplineComponent.SetTangentAtSplinePoint` _l_offsetspline_3 (- (`SplineComponent.GetNumberOfSplinePoints` _l_offsetspline_3) 1) (`SplineComponent.GetTangentAtDistanceAlongSpline` _l_base_spline_9 _returnvalue_3 "Local") "Local" false)))
            ;;[1 1 1] Setting the last point to a Curve (instead of linear) will avoid a corner point with wrong tangent generated
            (`SplineComponent.SetSplinePointType` _l_offsetspline _returnvalue_5 "Curve" true)
            (`KismetArrayLibrary.Array_Add` (`local.L_DistanceAtBasePoint`) (`SplineComponent.GetDistanceAlongSplineAtSplinePoint` _l_offsetspline _returnvalue_5))
            (`KismetArrayLibrary.Array_Add` (`local.L_IsCornerPoint`)))))
      (:`then_1`
        (return (make `/Game/fan_spawner/Structs/ST_OffsetSpline` (`local.L_OffsetSpline`) (`local.L_DistanceAtBasePoint`) (`local.L_IsCornerPoint`) (`local.L_IsUsingBaseSplineAsOffsetSpline`)))))))

(fn `SpawnInstanceItem`
  (params (BP_AutoSpawner :type "/Game/fan_spawner/Blueprints/Main_Blueprints/BP_Fan_Spawner Object Reference"))
  (locals (`custom ground` :type Boolean) (Local_BP_AutoSPawner :type "/Game/fan_spawner/Blueprints/Main_Blueprints/BP_Fan_Spawner Object Reference") (`L_chairs data table` :type "DataTable Object Reference") (`L_chairs to spawn` :type Integer :default 0) (L_Spawn_Sys :type Integer) (`Chair Transforms` :type "Array of Transform Structure") (`Chair Location` :type "Transform Structure"))
  (bind _local_bp_autospawner (`local.Local_BP_AutoSPawner`))
  (bind _local_bp_autospawner_2 (`local.Local_BP_AutoSPawner`))
  (bind _local_bp_autospawner_3 (`local.Local_BP_AutoSPawner`))
  (bind _fan_bp (`self.fan bp`))
  (bind _yaw (.yaw (`self.K2_GetActorRotation`)))
  (bind _add_to_existing_fan_bp (`/Game/fan_spawner/Blueprints/Main_Blueprints/BP_Fan_Spawner.Add to Existing Fan Bp` _local_bp_autospawner_3))
  (set `local.Local_BP_AutoSPawner` BP_AutoSpawner)
  (set `self.to spawn fan bp` (`self.K2_GetActorLocation` BP_AutoSpawner))
  (set `self.custom ground` (`/Game/fan_spawner/Blueprints/Main_Blueprints/BP_Fan_Spawner.custom ground distance` BP_AutoSpawner))
  (set `local.L_chairs data table` (`/Game/fan_spawner/Blueprints/Main_Blueprints/BP_Fan_Spawner.Chairs DataTable` BP_AutoSpawner))
  (set `local.L_chairs to spawn` (`KismetMathLibrary.Conv_ByteToInt` (`/Game/fan_spawner/Blueprints/Main_Blueprints/BP_Fan_Spawner.chairs to spawn` BP_AutoSpawner)))
  (set `local.L_Spawn_Sys` (`/Game/fan_spawner/Blueprints/Main_Blueprints/BP_Fan_Spawner.Spawn Sys` BP_AutoSpawner))
  (bind _out_row (`self.get first data table name` (`local.L_chairs data table`) (`local.L_chairs to spawn`)))
  (set `self.custom distance to ground` (`/Game/fan_spawner/Blueprints/Main_Blueprints/BP_Fan_Spawner.custom ground dis ` BP_AutoSpawner))
  (bind (_staticmesh _spawncolour _chairscale _chairrotaion _rowsdistanceonebehindoneanother _collumdistancesidebyside _chairrotoffset _chairlocoffset _chair_scale_overide) (break `/Game/fan_spawner/Structs/ST_SpawnItemInformation` _out_row))
  (set `self.scale chair` _chairscale)
  (set `self.offset Transform` (`KismetMathLibrary.MakeTransform` _chairlocoffset _chairrotoffset _chair_scale_overide))
  (set `self.chair scale` _chair_scale_overide)
  (switch `int` (`local.L_Spawn_Sys`)
    (:`0`
      (bind _returnvalue (+ _rowsdistanceonebehindoneanother (`/Game/fan_spawner/Blueprints/Main_Blueprints/BP_Fan_Spawner.cus spacer Y` _local_bp_autospawner_2)))
      (bind _returnvalue_2 (+ _collumdistancesidebyside (`/Game/fan_spawner/Blueprints/Main_Blueprints/BP_Fan_Spawner.cus spacer X` _local_bp_autospawner_2)))
      (bind _chair_transform (`self.Line Transform` (`local.Local_BP_AutoSPawner`) _returnvalue _returnvalue_2))
      (set `local.Chair Transforms` _chair_transform)
      (set `self.Rot Offset` 90.0))
    (:`1`
      (bind _chair_transforms (`/Game/fan_spawner/Blueprints/AutoUsed/BP_AutoSpawnerLibrary.Square Transform` (`local.Local_BP_AutoSPawner`) _chairrotaion _returnvalue _returnvalue_2))
      (set `local.Chair Transforms` _chair_transforms)
      (set `self.Rot Offset` 0.0)))
  (if (`/Game/fan_spawner/Blueprints/Main_Blueprints/BP_Fan_Spawner.dont add to existing` _local_bp_autospawner_3)
    (set `self.fan bp` null)
    (set `self.using existing fan bp` false)
    (else
      (`/Engine/EditorBlueprintResources/StandardMacros.IsValid` _add_to_existing_fan_bp
        (:`Is Valid`
          (set `self.fan bp` _add_to_existing_fan_bp)
          (set `self.using existing fan bp` true))
        (:`Is Not Valid`
          (set `self.using existing fan bp` false)))))
  (bind _returnvalue_3 (`self.custom ground dis` (`local.Chair Transforms`))
    (:`LoopBody`
      (`/Engine/EditorBlueprintResources/StandardMacros.IsValid` _fan_bp
        (:`Is Valid`
          (`/Game/fan_spawner/Blueprints/Main_Blueprints/BP_Fan_Spawner.tester` _local_bp_autospawner null false))
        (:`Is Not Valid`
          (bind _out_row_2 (`self.get first data table name` (`local.L_chairs data table`) (`local.L_chairs to spawn`)))
          (`self.AddInstanced` _out_row_2 (`local.Local_BP_AutoSPawner`))
          (`/Game/fan_spawner/Blueprints/Main_Blueprints/BP_Fan_Spawner.tester` _local_bp_autospawner (`self.fan bp`) true)))
      (switch `int` (`local.L_Spawn_Sys`)
        (:`0`
          ;[1 1 1] Line Editor
          (set `local.Chair Location` (`KismetMathLibrary.MakeTransform` (.location _returnvalue_3) (.rotation _returnvalue_3) (.scale (`self.offset Transform`)))))
        (:`1`
          ;[1 1 1] Square Editor
          (set `local.Chair Location` (`KismetMathLibrary.MakeTransform` (`KismetMathLibrary.RotateAngleAxis` (+ (.location _returnvalue_3) (.location (`self.offset Transform`))) _yaw (0.0 0.0 -1.0)) (`KismetMathLibrary.MakeRotator` 0.0 0.0 (- (+ (.yaw (.rotation _returnvalue_3)) (.yaw (.rotation (`self.offset Transform`)))) _yaw)) (.scale (`self.offset Transform`))))))
      (if (`self.using existing fan bp`)
        (set `local.Chair Location` (`KismetMathLibrary.MakeTransform` (+ (- (`self.K2_GetActorLocation` (`local.Local_BP_AutoSPawner`)) (`self.K2_GetActorLocation` (`self.fan bp`))) (.location (`local.Chair Location`))) (.rotation (`local.Chair Location`)) (.scale (`local.Chair Location`)))))
      (if (`/Game/fan_spawner/Blueprints/Main_Blueprints/BP_Fan_Spawner.Standing event (No Chairs)` (`local.Local_BP_AutoSPawner`))
        (`InstancedStaticMeshComponent.AddInstance` (`/Game/fan_spawner/Blueprints/AutoUsed/BP_fans.No Chair Placer` (`self.fan bp`)) (`local.Chair Location`))
        (else
          (bind _returnvalue_4 (`InstancedStaticMeshComponent.AddInstance` (`/Game/fan_spawner/Blueprints/AutoUsed/BP_fans.chair model` (`self.fan bp`)) (`local.Chair Location`)))
          (bind (_to_find_instane_with_colour _liner_color_out) (`/Game/fan_spawner/Blueprints/AutoUsed/BP_AutoSpawnerLibrary.get Color from Enum` _returnvalue_4 (`/Game/fan_spawner/Blueprints/Main_Blueprints/BP_Fan_Spawner.Spawn Color` (`local.Local_BP_AutoSPawner`)) (`/Game/fan_spawner/Blueprints/AutoUsed/BP_fans.chair model` (`self.fan bp`)) self))))
      (`/Game/fan_spawner/Blueprints/AutoUsed/BP_fans.get fan locations` (`self.fan bp`) (`self.offset Transform`) _liner_color_out (`/Game/fan_spawner/Blueprints/Main_Blueprints/BP_Fan_Spawner.Standing event (No Chairs)` (`local.Local_BP_AutoSPawner`)))
      (`self.K2_DestroyActor`))
    (:`Completed`
      (`/Game/fan_spawner/Blueprints/AutoUsed/BP_fans.set scale of chair` _fan_bp _chair_scale_overide))))

(fn `UserConstructionScript`
  (locals (Counter :type Integer)))